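; BP_Enemy0102 is an enemy Blueprint that issues one AI move order shortly after spawning.
; The construction script stores the first TargetPoint found as Target, and a non-looping BeginPlay timer calls MoveToLocation.
; That event passes the unit direction toward Target, rather than its position, as the SimpleMoveToLocation goal.
; Rotation smoothing and alternating timed moves are unconnected; Tick and MoveToLocation2 are empty.
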(event `self.ReceiveBeginPlay`
  (`KismetSystemLibrary.K2_SetTimer` null "MoveToLocation" 1.0))

(event `MoveToLocation2`)

(event `self.ReceiveTick`
  (params (DeltaSeconds :type "Float (single-precision)")))

(event `MoveToLocation`
  (`AIBlueprintHelperLibrary.SimpleMoveToLocation` (`self.GetController`) (`KismetMathLibrary.GetDirectionUnitVector` (`self.K2_GetActorLocation`) (`self.K2_GetActorLocation` (`self.Target`)))))

(fn `UserConstructionScript`
  (bind _outactors (`GameplayStatics.GetAllActorsOfClass` "/Script/Engine.TargetPoint"))
  (set `self.Target` (`|GetArrayItem` _outactors)))