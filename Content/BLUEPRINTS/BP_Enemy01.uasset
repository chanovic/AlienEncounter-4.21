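; BP_Enemy01 is an enemy that kills the player's BP_Robot on contact.
; A mesh hit from the robot calls PlayerDeath on the robot's GameMode reference, after a cast check on the current game mode.
; The construction script copies ControlPoints into the InterpToMovement component for its path.
; An alternative timer-driven AI patrol between two locations is left disconnected, with empty MoveToLocation events.
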(event `self.ReceiveBeginPlay`)

(event `MoveToLocation`)

(event `MoveToLocation2`)

(event `self.Enemy01Mesh.OnComponentHit`
  (params (HitComponent :type "PrimitiveComponent Object Reference") (OtherActor :type "Actor Object Reference") (OtherComp :type "PrimitiveComponent Object Reference") (NormalImpulse :type "Vector Structure") (Hit :type "HitResult Structure (by ref)"))
  (bind _asbp_robot (cast `/Game/BLUEPRINTS/BP_Robot` OtherActor))
  (cast `/Game/BLUEPRINTS/BP_GameMode` (`GameplayStatics.GetGameMode`))
  (`/Game/BLUEPRINTS/BP_GameMode.PlayerDeath` (`/Game/BLUEPRINTS/BP_Robot.GameMode` _asbp_robot)))

(fn `UserConstructionScript`
  (set `InterpToMovementComponent.ControlPoints` (`self.ControlPoints`) (`self.InterpToMovement`)))