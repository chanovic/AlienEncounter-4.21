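; Game mode that runs the countdown and handles death and respawn of the player's BP_Robot.
; A Delay on Tick decrements the GameInstance Timer about once a second and quits the game at zero.
; PlayerDeath explodes and hides the robot, then after a pause decrements Lifes and calls RespawnPlayer without checking remaining lives.
; RespawnPlayer spawns and possesses a new robot behind a reversed fade-to-black widget; the old robot is never destroyed.
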(event `self.ReceiveTick`
  (params (DeltaSeconds :type "Float (single-precision)"))
  (`KismetSystemLibrary.Delay` 1.0)
  (bind _asbp_game_instance (cast `/Game/BLUEPRINTS/BP_GameInstance` (`GameplayStatics.GetGameInstance`)))
  (set `/Game/BLUEPRINTS/BP_GameInstance.Timer` (- (`/Game/BLUEPRINTS/BP_GameInstance.Timer` _asbp_game_instance) 1) _asbp_game_instance)
  (if (== (`/Game/BLUEPRINTS/BP_GameInstance.Timer` _asbp_game_instance) 0)
    (`KismetSystemLibrary.QuitGame` null "Quit")))

(event `RespawnPlayer`
  (bind _returnvalue (`|SpawnActorFromClass` "/Game/BLUEPRINTS/BP_Robot.BP_Robot_C" (`self.PlayerSpawnTransform`) "AlwaysSpawn" "OverrideRootScale" null null))
  (bind _returnvalue_2 (`|CreateWidget` "/Game/WIDGETS/Widget_Death.Widget_Death_C"))
  (`UserWidget.AddToViewport` _returnvalue_2 0)
  (`UserWidget.PlayAnimation` _returnvalue_2 (`/Game/WIDGETS/Widget_Death.FadeBlackAnim` _returnvalue_2) 0.0 1 "Reverse" 0.2)
  (`Controller.Possess` (`GameplayStatics.GetPlayerController` 0) _returnvalue))

(event `PlayerDeath`
  (bind _asbp_robot (cast `/Game/BLUEPRINTS/BP_Robot` (`GameplayStatics.GetPlayerCharacter` 0)))
  (`GameplayStatics.SpawnEmitterAtLocation` "/Game/StarterContent/Particles/P_Explosion.P_Explosion" (`self.K2_GetActorLocation` _asbp_robot))
  (`SceneComponent.SetVisibility` (`Actor.RootComponent` _asbp_robot) false true)
  (set `/Game/BLUEPRINTS/BP_Robot.bIsDestroyed?` true _asbp_robot)
  (bind _asbp_game_instance (cast `/Game/BLUEPRINTS/BP_GameInstance` (`GameplayStatics.GetGameInstance`)))
  (`KismetSystemLibrary.Delay` 1.4)
  (set `/Game/BLUEPRINTS/BP_GameInstance.Lifes` (- (`/Game/BLUEPRINTS/BP_GameInstance.Lifes` _asbp_game_instance) 1) _asbp_game_instance)
  (`self.RespawnPlayer` (`/Game/BLUEPRINTS/BP_Robot.GameMode` _asbp_robot))
  (bind _returnvalue (`|CreateWidget` "/Game/WIDGETS/Widget_Death.Widget_Death_C"))
  (`UserWidget.AddToViewport` _returnvalue 0))

(fn `UserConstructionScript`)