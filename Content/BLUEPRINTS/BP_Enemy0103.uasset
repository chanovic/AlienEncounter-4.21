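; BP_Enemy0103 is an enemy that travels along a track's spline and kills the player robot on contact.
; When active at BeginPlay, a timeline with duration-scaled play rate drives its swept movement along SplineEnemy01 from TrackRef.
; Pitch and yaw come from the spline's start, with a fixed sideways roll.
; A mesh hit on BP_Robot calls PlayerDeath through the robot's GameMode reference.
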(event `self.ReceiveBeginPlay`
  (if (`self.Enemy01Active`)
    (`self.MoveEnemy01`)))

(event `MoveEnemy01`
  (bind (_returnvalue_roll _returnvalue_pitch _returnvalue_yaw) (`KismetMathLibrary.BreakRotator` (`SplineComponent.GetRotationAtDistanceAlongSpline` (`/Game/BLUEPRINTS/BP_TrackEnemy01.SplineEnemy01` (`self.TrackRef`)) 0.0 "World")))
  (`TimelineComponent.SetPlayRate` (`self.Enemy01Timeline`) (/ 1.0 (`self.Duration`)))
  (`TimelineComponent.SetNewTime` (`self.Enemy01Timeline`) (`self.Enemy01StartOffset`))
  (bind (_direction _alpha) (`Timeline|Enemy01Timeline` :!via `PlayFromStart`)
    (:`Update`
      (set `self.Alpha` _alpha)
      (`self.K2_SetActorLocationAndRotation` (`SplineComponent.GetLocationAtDistanceAlongSpline` (`/Game/BLUEPRINTS/BP_TrackEnemy01.SplineEnemy01` (`self.TrackRef`)) (`KismetMathLibrary.Lerp` 0.0 (`SplineComponent.GetSplineLength` (`/Game/BLUEPRINTS/BP_TrackEnemy01.SplineEnemy01` (`self.TrackRef`))) (`self.Alpha`)) "World") (`KismetMathLibrary.MakeRotator` 90.0 _returnvalue_pitch _returnvalue_yaw) true))))

(event `self.Enemy01Mesh.OnComponentHit`
  (params (HitComponent :type "PrimitiveComponent Object Reference") (OtherActor :type "Actor Object Reference") (OtherComp :type "PrimitiveComponent Object Reference") (NormalImpulse :type "Vector Structure") (Hit :type "HitResult Structure (by ref)"))
  (bind _asbp_robot (cast `/Game/BLUEPRINTS/BP_Robot` OtherActor))
  (cast `/Game/BLUEPRINTS/BP_GameMode` (`GameplayStatics.GetGameMode`))
  (`/Game/BLUEPRINTS/BP_GameMode.PlayerDeath` (`/Game/BLUEPRINTS/BP_Robot.GameMode` _asbp_robot)))

(fn `UserConstructionScript`)